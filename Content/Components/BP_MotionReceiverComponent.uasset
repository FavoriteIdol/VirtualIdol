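; Component that receives Remocapp motion capture data over OSC, covering control transforms and face morph values.
; On BeginPlay it starts an OSC server on a configurable port and sizes the face morph array.
; Each bundle's messages are routed by address: transforms are scaled 100x in location, converted from quaternions and broadcast per control, while morph values fill the array by index.
; Finished dispatchers fire after every bundle, passing along the face array.
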(event `self.ReceiveBeginPlay`
  (bind _returnvalue (`OSCManager.CreateOSCServer` "0.0.0.0" (`self.ReceiverPortNumber`) false true "" self))
  (bind _output_get (set `self.ServerInstance` _returnvalue))
  (add `OSCServer.OnOscBundleReceived` _output_get (delegate `OnOscBundleReceived`))
  (`KismetArrayLibrary.Array_Resize` (`self.FaceMorphData`) (`self.FaceMorphCount`)))

(event `OnOscBundleReceived`
  (params (Bundle :type "OSCBundle Structure (by ref)") (IPAddress :type String) (Port :type Integer))
  (bind _receivedmessage (`self.ReceivedMessage`))
  (bind _returnvalue (`OSCManager.GetMessagesFromBundle` Bundle))
  (for _array_element _returnvalue
    (bind _output_get (set `self.ReceivedMessage` _array_element))
    (bind _returnvalue_2 (`OSCManager.GetOSCMessageAddress` _output_get))
    (bind _returnvalue_3 (`OSCManager.GetOSCAddressFullPath` _returnvalue_2))
    (switch `string` _returnvalue_3
      (:`/Remocapp/UE`
        (bind (_controlindex _controltransform) (`self.RetrieveControlData` _receivedmessage))
        (`self.OnControlTransformReceived` _controlindex _controltransform))
      (:`/Remocapp/UE/Face`
        (`self.RetrieveFaceMorphData` _receivedmessage))))
  (`self.OnRetrievingControlsDataFinished`)
  (`self.OnRetrievingFaceDataFinished` (`self.FaceMorphData`)))

(fn `RetrieveControlData`
  (params (Message :type "OSCMessage Structure"))
  (returns (ControlIndex :type Integer) (ControlTransform :type "Transform Structure"))
  (locals (ReceivedControlIndex :type Integer :default 0))
  (bind (_value _returnvalue) (`OSCManager.GetInt32` Message))
  (set `local.ReceivedControlIndex` _value)
  (if _returnvalue
    (bind _values (`OSCManager.GetAllFloats` Message))
    (return (`local.ReceivedControlIndex`) (`KismetMathLibrary.MakeTransform` (* (`KismetMathLibrary.MakeVector` (`|GetArrayItem` _values 1) (`|GetArrayItem` _values 2) (`|GetArrayItem` _values 3)) 100.0) (`KismetMathLibrary.Quat_Rotator` (`KismetMathLibrary.MakeQuat` (`|GetArrayItem` _values 4) (`|GetArrayItem` _values 5) (`|GetArrayItem` _values 6) (`|GetArrayItem` _values 7)))))))

(fn `RetrieveFaceMorphData`
  (params (Message :type "OSCMessage Structure"))
  (locals (ReceivedMorphIndex :type Integer))
  (bind (_value _returnvalue) (`OSCManager.GetInt32` Message))
  (set `local.ReceivedMorphIndex` _value)
  (if _returnvalue
    (bind _value_2 (`OSCManager.GetFloat` Message 3))
    (`KismetArrayLibrary.Array_Set` (`self.FaceMorphData`) (`local.ReceivedMorphIndex`) _value_2)
    (return)))
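; BP_VFX-Fever-A_Christrmas is a self-destroying VFX actor that plays a Niagara cold sparks stream, named as the Christmas variant of a Fever effect.
; BeginPlay sets the system's User.DensityScale from JswDensityScale, and Tick re-applies that variable every frame.
; Chained timers zero the density after three seconds, then destroy the actor one second later.
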(event `self.ReceiveBeginPlay`
  (`NiagaraComponent.SetNiagaraVariableFloat` (`self.NS_ColdSparks_Stream08_JSW`) "User.DensityScale" (`self.jswDensityScale`))
  (`KismetSystemLibrary.K2_SetTimerDelegate` (delegate `SetValue`) 3.0))

(event `SetValue`
  (set `self.jswDensityScale` 0.0)
  (`KismetSystemLibrary.K2_SetTimerDelegate` (delegate `Destroy`) 1.0))

(event `Destroy`
  (`self.K2_DestroyActor`))

(event `self.ReceiveTick`
  (params (DeltaSeconds :type "Float (single-precision)"))
  (bind _output_get (set `self.jswDensityScale` (`self.jswDensityScale`)))
  (`NiagaraComponent.SetNiagaraVariableFloat` (`self.NS_ColdSparks_Stream08_JSW`) "User.DensityScale" _output_get))

(fn `UserConstructionScript`)
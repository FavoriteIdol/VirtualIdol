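; BP_NS_Sparkler_blast is a VFX actor for a sparkler blast effect built on four Niagara components.
; A SetValue event zeroes the Spark_amount parameter on all four components, and a Destroy event removes the actor.
; Timers meant to fire these events after a short delay are disconnected, and BeginPlay is empty, so the graph itself never triggers the fade-out or cleanup.
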(event `self.ReceiveBeginPlay`)

(event `Destroy`
  (`self.K2_DestroyActor`))

(event `SetValue`
  (`FXSystemComponent.SetFloatParameter` (`self.NS_Sparkler_blast`) "Spark_amount" 0.0)
  (`FXSystemComponent.SetFloatParameter` (`self.NS_Sparkler_blast1`) "Spark_amount" 0.0)
  (`FXSystemComponent.SetFloatParameter` (`self.NS_Sparkler_blast2`) "Spark_amount" 0.0)
  (`FXSystemComponent.SetFloatParameter` (`self.NS_Sparkler_blast3`) "Spark_amount" 0.0))

(fn `UserConstructionScript`)
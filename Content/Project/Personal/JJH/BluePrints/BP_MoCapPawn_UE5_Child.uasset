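; Motion-capture pawn child Blueprint that adds virtual-widget controls, a dance trigger and an interviewee hotkey for multiplayer.
; On BeginPlay the host's local player gets a WBP_VirtualWidget_KMK, shared with the VirtualKMK component and game instance.
; C, host-only, changes that widget and calls VirtualKMK's CallGMShowServer.
; Key 1 sets CanDance through a server-to-multicast event chain, while I calls the Auditorium GameState's set-interviewee RPC.
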(event `self.ReceiveBeginPlay`
  (bind _returnvalue (`GameplayStatics.GetPlayerController` 0))
  (`parent.ReceiveBeginPlay`)
  (if (and (`self.HasAuthority` _returnvalue) (`Controller.IsLocalPlayerController` _returnvalue))
    (bind _returnvalue_2 (`|CreateWidget` "/Game/Project/Personal/KMK/UI/WBP_VirtualWidget_KMK.WBP_VirtualWidget_KMK_C"))
    (`UserWidget.AddToViewport` _returnvalue_2 0)
    (`WidgetBlueprintLibrary.SetInputMode_GameAndUIEx` _returnvalue null)
    (bind _output_get (set `Virtual_KMK.virtualWidget` _returnvalue_2 (`self.Virtual_KMK`)))
    (bind _asvirtual_game_instance_kmk (cast `VirtualGameInstance_KMK` (`GameplayStatics.GetGameInstance`)))
    (`VirtualGameInstance_KMK.SetWidget` _asvirtual_game_instance_kmk _output_get)))

(event `Key|C`
  (params (Key :type "Key Structure")))

(event `Key|C`
  (params (Key :type "Key Structure"))
  (bind _virtual_kmk (`self.Virtual_KMK`))
  (:`Pressed`
    (if (and (`self.HasAuthority`) (`self.IsLocallyControlled`))
      (`Audience_KMK.ChangeVirtualWidget` (`Virtual_KMK.virtualWidget` _virtual_kmk))
      (`Virtual_KMK.CallGMShowServer` _virtual_kmk))))

(event `Key|One`
  (params (Key :type "Key Structure"))
  (:`Pressed`
    (`self.ServerPlayAnimation`)))

(event `MulticastPlayAniation`
  (set `self.bCanDance` true))

(event `ServerPlayAnimation`
  (`self.MulticastPlayAniation`))

(event `Key|I`
  (params (Key :type "Key Structure"))
  (:`Pressed`
    (bind _ashsw_game_state_auditorium (cast `HSW_GameState_Auditorium` (`GameplayStatics.GetGameState`))
      (:`then`
        (`HSW_GameState_Auditorium.ServerRPC_SetInterviewee` _ashsw_game_state_auditorium)
        (`KismetSystemLibrary.PrintString` "ㅋㅋ"))
      (:`CastFailed`
        (`KismetSystemLibrary.PrintString` "Fail!")))))

(fn `UserConstructionScript`
  (`parent.UserConstructionScript`))
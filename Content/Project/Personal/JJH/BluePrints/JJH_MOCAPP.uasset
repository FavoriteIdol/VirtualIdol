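; Pawn or Character Blueprint that drives its skeletal mesh from received motion data through a Control Rig component.
; The rig takes initial bone transforms from the mesh's sockets and outputs to that mesh.
; On an authoritative, locally controlled instance, received control transforms are offset by the mesh's starting world location and set on the indexed controls through custom event 1231234.
; The rig updates when the receiver finishes retrieving control data.
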(event `self.ControlRig.OnPreConstructionDelegate`
  (params (Component :type "ControlRigComponent Object Reference"))
  (bind _mesh (`self.Mesh`))
  (for _array_element (`SceneComponent.GetAllSocketNames` _mesh)
    (if (`SceneComponent.DoesSocketExist` _mesh _array_element)
      (`ControlRigComponent.SetInitialBoneTransform` (`self.ControlRig`) _array_element (`SceneComponent.GetSocketTransform` _mesh _array_element "RTS_Component") "ComponentSpace" true))))

(event `self.ControlRig.OnPostInitializeDelegate`
  (params (Component :type "ControlRigComponent Object Reference"))
  (`ControlRigComponent.AddMappedCompleteSkeletalMesh` (`self.ControlRig`) (`self.Mesh`) "Output"))

(event `self.ReceiveBeginPlay`
  (bind _bp_motionreceivercomponent (`self.BP_MotionReceiverComponent`))
  (set `self.MeshInitialLocation` (`SceneComponent.K2_GetComponentLocation` (`self.Mesh`)))
  (add `/ReMoCapp/Components/BP_MotionReceiverComponent.OnControlTransformReceived` _bp_motionreceivercomponent (delegate `ControlTransformReceived`))
  (add `/ReMoCapp/Components/BP_MotionReceiverComponent.OnRetrievingControlsDataFinished` _bp_motionreceivercomponent (delegate `RetrievingControlsDataFinished`)))

(event `RetrievingControlsDataFinished`
  (`ControlRigComponent.Update` (`self.ControlRig`) 0.0))

(event `ControlTransformReceived`
  (params (ControlIndex :type Integer) (ControlTransform :type "Transform Structure"))
  (if (and (`self.HasAuthority`) (`self.IsLocallyControlled`))
    (`self.1231234` ControlIndex ControlTransform)))

(event `1231234`
  (params (NewParam :type Integer) (NewParam2 :type "Transform Structure"))
  (bind _controlrig (`self.ControlRig`))
  (`/Engine/EditorBlueprintResources/StandardMacros.IsValid` _controlrig
    (:`Is Valid`
      (`ControlRigComponent.SetControlTransform` _controlrig (`|GetArrayItem` (`self.Rig Control Names`) NewParam) (`KismetMathLibrary.MakeTransform` (+ (.location NewParam2) (`self.MeshInitialLocation`)) (.rotation NewParam2) (.scale NewParam2)) "WorldSpace"))))

(fn `UserConstructionScript`)
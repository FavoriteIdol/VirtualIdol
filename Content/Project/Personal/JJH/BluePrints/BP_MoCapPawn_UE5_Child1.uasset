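; Child mocap pawn that drives a VRM avatar in a virtual stage show with an interview feature.
; BeginPlay creates the virtual widget for the local authority player and shares it with VirtualKMK and the game instance.
; C starts the show with delayed music; I requests an interviewee through the auditorium game state.
; Construction wires BPVrmAnimControlComponent for look-at and forced blinks, while a timeline loop drives randomly timed blink morph targets.
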(event `self.ReceiveBeginPlay`
  (bind _returnvalue (`GameplayStatics.GetPlayerController` 0))
  (`parent.ReceiveBeginPlay`)
  (if (and (`self.HasAuthority` _returnvalue) (`Controller.IsLocalPlayerController` _returnvalue))
    (bind _returnvalue_2 (`|CreateWidget` "/Game/Project/Personal/KMK/UI/WBP_VirtualWidget_KMK.WBP_VirtualWidget_KMK_C"))
    (`UserWidget.AddToViewport` _returnvalue_2 0)
    (`WidgetBlueprintLibrary.SetInputMode_GameAndUIEx` _returnvalue null)
    (bind _output_get (set `Virtual_KMK.virtualWidget` _returnvalue_2 (`self.Virtual_KMK`)))
    (bind _asvirtual_game_instance_kmk (cast `VirtualGameInstance_KMK` (`GameplayStatics.GetGameInstance`)))
    (`VirtualGameInstance_KMK.SetWidget` _asvirtual_game_instance_kmk _output_get)
    (if (`self.bUseArkitMorphCurveName`)
      _)))

(event `Key|C`
  (params (Key :type "Key Structure")))

(event `Key|C`
  (params (Key :type "Key Structure"))
  (bind _virtual_kmk (`self.Virtual_KMK`))
  ;[1 1 1] 무대시작
  (:`Pressed`
    (if (and (`self.HasAuthority`) (`self.IsLocallyControlled`))
      (`Audience_KMK.ChangeVirtualWidget` (`Virtual_KMK.virtualWidget` _virtual_kmk))
      (`Virtual_KMK.CallGMShowServer` _virtual_kmk)
      (bind _output_get (set `self.SoundWav` "/Game/Project/Personal/HSW/Resources/WavFile/howsweet.howsweet"))
      (`KismetSystemLibrary.Delay` 6.0)
      (`GameplayStatics.PlaySound2D` _output_get 1.0 1.0 0.0 null null))))

(event `Key|I`
  (params (Key :type "Key Structure"))
  ;[1 1 1] 인터뷰
  (:`Pressed`
    (bind _ashsw_game_state_auditorium (cast `HSW_GameState_Auditorium` (`GameplayStatics.GetGameState`))
      (:`then`
        (`HSW_GameState_Auditorium.ServerRPC_SetInterviewee` _ashsw_game_state_auditorium)
        (`KismetSystemLibrary.PrintString` "ㅋㅋ"))
      (:`CastFailed`
        (`KismetSystemLibrary.PrintString` "Fail!")))))

(event `BeginBlink`
  (bind _skeletalmesh (`self.SkeletalMesh`))
  ;[1 1 1] Blink
  (`/Engine/EditorBlueprintResources/StandardMacros.DoOnce` false
    (:`Completed`
      (`self.VrmAssetList`
        (:`then`
          (`|ExecutionSequence` :!label _label
            (:`then_2`
              (`|ExecutionSequence`
                (:`then_0`
                  (goto _label_2 :!via `Reset`))
                (:`then_1`
                  (`KismetSystemLibrary.RetriggerableDelay` (`KismetMathLibrary.RandomFloatInRange` 1.0 6.0))
                  (`/Engine/EditorBlueprintResources/StandardMacros.DoOnce` false :!label _label_2
                    (:`Completed`
                      (if (`self.bEnableBlink`) :!label _label_3
                        (bind (_direction _newtrack_0) (`Timeline|Timeline` :!via `PlayFromStart`)
                          (:`Update`
                            (if (not (`/VRM4U/Util/BaseCharacter/Misc/BP_VrmAnimControlComponent.AnimStopFrame` (`self.BP_VrmAnimControlComponent`)))
                              (for _array_element (`VrmMetaObject.BlendShapeGroup` (`VrmAssetListObject.VrmMetaObject` (`self.VRMAssetList`)))
                                (bind (_name _blendshape) (break `VrmBlendShapeGroup` _array_element))
                                (if (`KismetStringLibrary.EqualEqual_StrStr` _name "Blink")
                                  (`|ExecutionSequence`
                                    (:`then_0`
                                      (for _array_element_2 _blendshape
                                        (`SkeletalMeshComponent.SetMorphTarget` (`self.SkeletalMesh`) (`KismetStringLibrary.Conv_StringToName` (`.morphTargetName` (break `VrmBlendShape` _array_element_2))) _newtrack_0 true)))
                                    (:`then_1`
                                      (if (`SceneComponent.IsVisible` _skeletalmesh)
                                        (`SkeletalMeshComponent.SetMorphTarget` _skeletalmesh "Face.M_F00_000_Fcl_EYE_Close" _newtrack_0 true)))
                                    (:`then_2`
                                      (break)))))))
                          (:`Finished`
                            (`|ExecutionSequence`
                              (:`then_0`
                                (goto _label))
                              (:`then_1`
                                (`SkeletalMeshComponent.ClearMorphTargets` (`self.SkeletalMesh`))))))))))))))
        (:`else`)))))

(event `ForceBlink`
  ;[1 1 1] Blink
  (goto _label_2))

(event `SetBlinkEnable`
  (params (bEnable :type Boolean))
  ;[1 1 1] Blink
  (if (!= bEnable (`self.bEnableBlink`))
    (set `self.bEnableBlink` bEnable)
    (goto _label_3)))

(event `SetLookAtForce`
  (params (LookAtForce :type "Float (double-precision)"))
  (`/VRM4U/Util/BaseCharacter/Misc/BP_VrmAnimControlComponent.SetLookAtForce` (`self.BP_VrmAnimControlComponent`) LookAtForce))

(event `SetLookAtTarget`
  (params (TargetLocation :type "Vector Structure"))
  (`/VRM4U/Util/BaseCharacter/Misc/BP_VrmAnimControlComponent.SetLookAtTarget` (`self.BP_VrmAnimControlComponent`) TargetLocation))

(event `SetLookAtType`
  (params (Eye :type Boolean :default true) (Head :type Boolean :default true))
  (`/VRM4U/Util/BaseCharacter/Misc/BP_VrmAnimControlComponent.SetLookAtType` (`self.BP_VrmAnimControlComponent`) Eye Head))

(fn `UserConstructionScript`
  (bind _bp_vrmanimcontrolcomponent (`self.BP_VrmAnimControlComponent`))
  (`parent.UserConstructionScript`)
  (`/VRM4U/Util/BaseCharacter/Misc/BP_VrmAnimControlComponent.SetSkeleton` _bp_vrmanimcontrolcomponent (`self.Mesh`) (`self.SkeletalMesh`) (`self.VrmAssetList`))
  (add `/VRM4U/Util/BaseCharacter/Misc/BP_VrmAnimControlComponent.OnForceBlink` _bp_vrmanimcontrolcomponent (`|CreateDelegate` :!event `ForceBlink`)))
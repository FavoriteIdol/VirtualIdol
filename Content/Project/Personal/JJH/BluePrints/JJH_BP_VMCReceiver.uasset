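; VMC receiver actor that runs an OSC server on a configurable IP and port to feed live motion data to VRM4U.
; Each message becomes an axis-swapped, centimeter-scaled transform in bone and raw maps, pushed per port to the VRM4U anim subsystem.
; Blend shape values are only stored locally.
; Server creation also triggers EUB_VMCTick editor ticking by console command; DebugDraw shows bones as cubes.
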(event `ServerStop`
  (`|ExecutionSequence`
    (:`then_0`
      (bind _ocsserver (`self.OCSServer`)
        (:`then`
          (`OSCServer.Stop` _ocsserver)
          (remove `OSCServer.OnOscMessageReceived` _ocsserver (`|CreateDelegate` :!event `CustomEvent_0`)))
        (:`else`)))
    (:`then_1`
      (set `self.OCSServer` null))
    (:`then_2`
      (`VRM4U_AnimSubsystem.Clear` (subsystem `VRM4U_AnimSubsystem`))
      (`BlueprintMapLibrary.Map_Clear` (`self.BoneInfo`))
      (`BlueprintMapLibrary.Map_Clear` (`self.BoneInfo_raw`)))))

(event `CreateServer`
  (params (ReceiveIPAddress :type String) (Port :type Integer))
  (bind _ocsserver (`self.OCSServer`))
  (`|ExecutionSequence`
    (:`then_0`
      (set `self.Receive IPAddress` ReceiveIPAddress))
    (:`then_1`
      (set `self.Port` Port))
    (:`then_2`
      (`|ExecutionSequence` :!label _label
        (:`then_0`
          (bind _ocsserver_2 (`self.OCSServer`)
            (:`then`
              (`OSCServer.Stop` _ocsserver_2)
              (clear `OSCServer.OnOscMessageReceived` _ocsserver_2)
              (clear `OSCServer.OnOscBundleReceived` _ocsserver_2))
            (:`else`)))
        (:`then_1`
          (bind _returnvalue (`OSCManager.CreateOSCServer` (`self.Receive IPAddress`) (`self.Port`) false true "" self))
          (bind _output_get (set `self.OCSServer` _returnvalue))
          (`self.OnCreateOCSServer` _output_get))
        (:`then_3`
          (`OSCManager.OSCAddressFromObjectPath` _ocsserver))
        (:`then_4`
          (add `OSCServer.OnOscMessageReceived` _ocsserver (delegate `CustomEvent_0`)))
        (:`then_5`
          (`KismetSystemLibrary.ExecuteConsoleCommand` "ke EUB_VMCTick_C SetVMCEditorTick true" null))
        (:`then_6`
          (if (and (== (`self.bCallBackEUW`) false) (== (`self.bCallBeginPlay`) false))
            (`KismetSystemLibrary.PrintString` "error. \nPlace EUB_VMCTick in level")))))))

(event `ServerListen`
  (set `self.bCallBackEUW` false)
  (goto _label))

(event `self.ReceiveBeginPlay`
  (set `self.bCallBeginPlay` true)
  (`|ExecutionSequence`
    (:`then_0`
      (goto _label))
    (:`then_1`
      (if (`self.bDebugDraw`)
        (for _ (range 34)
          (bind _returnvalue (`AddComponent|NODE_AddStaticMeshComponent-0` :`RelativeTransform` (`KismetMathLibrary.MakeTransform` (0.0 0.0 0.0) (struct) (0.1 0.1 0.1))))
          (`KismetArrayLibrary.Array_AddUnique` (`self.StaticMesh_Cube`) _returnvalue)
          (`StaticMeshComponent.SetStaticMesh` _returnvalue "/Engine/BasicShapes/Cube.Cube"))))))

(event `OnCreateOCSServerDummy`
  (params (OCSServer :type "OSCServer Object Reference")))

(event `self.ReceiveTick`
  (params (DeltaSeconds :type "Float (single-precision)"))
  (bind _boneinfo (`self.BoneInfo`))
  (if (`self.bDebugDraw`)
    (`|ExecutionSequence`
      (:`then_1`
        (bind _keys (`BlueprintMapLibrary.Map_Keys` _boneinfo))
        (bind _values (`BlueprintMapLibrary.Map_Values` _boneinfo))
        (for (_array_element _array_index) _keys
          (`SceneComponent.K2_SetRelativeTransform` (`|GetArrayItem` (`self.StaticMesh_Cube`) _array_index) (`KismetMathLibrary.MakeTransform` (.location (`|GetArrayItem` _values _array_index)) (.rotation (`|GetArrayItem` _values _array_index)) (0.1 0.1 0.1)) false false))))))

(event `CustomEvent_1`
  (params (AddressPattern :type "OSCAddress Structure (by ref)") (Message :type "OSCMessage Structure (by ref)") (IPAddress :type String) (Port :type Integer))
  (if true
    _))

(event `CustomEvent_0`
  (params (Message :type "OSCMessage Structure (by ref)") (IPAddress :type String) (Port :type Integer))
  (bind _returnvalue (subsystem `VRM4U_AnimSubsystem`))
  (bind _port (`self.Port`))
  (bind _returnvalue_2 (`KismetMathLibrary.MakeTransform` (`self.tmpPos`) (`self.tmpRot`) (`self.tmpScale`)))
  (`|ExecutionSequence`
    (:`then_2`
      (`|ExecutionSequence`
        (:`then_0`
          (bind _returnvalue_3 (`OSCManager.GetOSCMessageAddress` Message))
          (bind _returnvalue_4 (`OSCManager.GetOSCAddressFullPath` _returnvalue_3))
          (bind _returnvalue_5 (`OSCManager.GetOSCAddressContainers` _returnvalue_3))
          (bind _returnvalue_6 (`OSCManager.GetOSCAddressMethod` _returnvalue_3))
          (bind _returnvalue_7 (`OSCManager.GetOSCAddressContainerPath` _returnvalue_3))
          (bind _values (`OSCManager.GetAllStrings` Message))
          (if (== (`KismetArrayLibrary.Array_Length` _values) 0)
            (set `self.tmpStr` "")
            (else
              (set `self.tmpStr` (`|GetArrayItem` _values)))))
        (:`then_3`
          (`|ExecutionSequence`
            (:`then_0`
              (set `self.tmpRot` (struct))
              (set `self.tmpPos` (0.0 0.0 0.0))
              (set `self.tmpScale` (1.0 1.0 1.0)))
            (:`then_1`
              (bind _values_2 (`OSCManager.GetAllStrings` Message))
              (`|ExecutionSequence`
                (:`then_0`
                  (bind _values_3 (`OSCManager.GetAllFloats` Message))
                  (`|ExecutionSequence`
                    (:`then_0`
                      (bind _returnvalue_8 (`KismetArrayLibrary.Array_Length` _values_3))
                      (if (>= _returnvalue_8 7)
                        (set `self.tmpPos` (* (* (`KismetMathLibrary.MakeVector` (`|GetArrayItem` _values_3) (`|GetArrayItem` _values_3 2) (`|GetArrayItem` _values_3 1)) (-1.0 1.0 1.0)) 100.0))
                        (set `self.tmpRot` (`KismetMathLibrary.Quat_Rotator` (`KismetMathLibrary.MakeQuat` (* (`|GetArrayItem` _values_3 3) -1.0) (`|GetArrayItem` _values_3 5) (`|GetArrayItem` _values_3 4) (`|GetArrayItem` _values_3 6))))))
                    (:`then_1`
                      (if (>= _returnvalue_8 13)
                        (bind _returnvalue_9 (`KismetMathLibrary.MakeVector` (`|GetArrayItem` _values_3 10) (`|GetArrayItem` _values_3 11) (`|GetArrayItem` _values_3 12)))
                        (if (> (`KismetMathLibrary.VSize` _returnvalue_9) 0.0)
                          (set `self.tmpScale` _returnvalue_9)
                          (else
                            (set `self.tmpScale` (1.0 1.0 1.0))))))
                    (:`then_2`
                      (if (== _returnvalue_8 1)
                        (set `self.tmpPos` (`KismetMathLibrary.Conv_DoubleToVector` (`|GetArrayItem` _values_3)))))))
                (:`then_1`
                  (`|ExecutionSequence`
                    (:`then_0`
                      (if (== _returnvalue_4 "/VMC/Ext/Bone/Pos")
                        (bind _output (`|GetArrayItem` _values_2))
                        (`BlueprintMapLibrary.Map_Add` (`self.BoneInfo`) _output _returnvalue_2)))
                    (:`then_1`
                      (`BlueprintMapLibrary.Map_Add` (`self.BoneInfo_raw`) (`KismetStringLibrary.Concat_StrStr` _returnvalue_4 ":" "" "" (`self.tmpStr`)) _returnvalue_2))))
                (:`then_2`
                  (if (== _returnvalue_4 "/VMC/Ext/Blend/Val")
                    (`BlueprintMapLibrary.Map_Add` (`self.BlendShape`) _output (.x (`self.tmpPos`)))))
                (:`then_3`
                  (`VRM4U_AnimSubsystem.SetBoneTransform` _returnvalue _port (`self.BoneInfo`))
                  (`VRM4U_AnimSubsystem.SetRawData` _returnvalue _port (`self.BoneInfo_raw`)))))))))))

(fn `UserConstructionScript`
  (bind _addresstable (`VrmNetworkBPFunctionLibrary.VRMGetIPAddressTable`))
  (set `self.AddressTable` _addresstable))
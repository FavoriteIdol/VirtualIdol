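; BP_MoCapPawn_UE5_Child_HSW is a motion-capture pawn child with host-side keyboard controls for a virtual auditorium show.
; On BeginPlay the local authority creates the virtual widget, registers it with the game instance and caches all dummy actors.
; Keys start the show with delayed music, request an interviewee via GameState, reset an audience member's fever, spawn VFX and toggle dummy throwing.
; The server-to-multicast dance event is never triggered within this graph.
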(event `self.ReceiveBeginPlay`
  (bind _returnvalue (`GameplayStatics.GetPlayerController` 0))
  (`parent.ReceiveBeginPlay`)
  (if (and (`self.HasAuthority` _returnvalue) (`Controller.IsLocalPlayerController` _returnvalue))
    (bind _returnvalue_2 (`|CreateWidget` "/Game/Project/Personal/KMK/UI/WBP_VirtualWidget_KMK.WBP_VirtualWidget_KMK_C"))
    (`UserWidget.AddToViewport` _returnvalue_2 0)
    (`WidgetBlueprintLibrary.SetInputMode_GameAndUIEx` _returnvalue null)
    (bind _output_get (set `Virtual_KMK.virtualWidget` _returnvalue_2 (`self.Virtual_KMK`)))
    (bind _asvirtual_game_instance_kmk (cast `VirtualGameInstance_KMK` (`GameplayStatics.GetGameInstance`)))
    (`VirtualGameInstance_KMK.SetWidget` _asvirtual_game_instance_kmk _output_get)
    (bind _outactors (`GameplayStatics.GetAllActorsOfClass` "/Game/Project/Personal/KMK/Blueprint/BP_Dummy.BP_Dummy_C"))
    (set `self.Dummies` _outactors)))

(event `Key|C`
  (params (Key :type "Key Structure")))

(event `Key|C`
  (params (Key :type "Key Structure"))
  (bind _virtual_kmk (`self.Virtual_KMK`))
  (:`Pressed`
    (if (and (`self.HasAuthority`) (`self.IsLocallyControlled`))
      (`Audience_KMK.ChangeVirtualWidget` (`Virtual_KMK.virtualWidget` _virtual_kmk))
      (`Virtual_KMK.CallGMShowServer` _virtual_kmk)
      (bind _output_get (set `self.SoundWav` "/Game/Project/Personal/HSW/Resources/WavFile/howsweet.howsweet"))
      (`KismetSystemLibrary.Delay` 6.0)
      (`GameplayStatics.PlaySound2D` _output_get 1.0 1.0 0.0 null null))))

(event `MulticastPlayAniation`
  (set `self.bCanDance` true))

(event `Key|I`
  (params (Key :type "Key Structure"))
  ;[1 1 1] Keyboard Binding : I 인터뷰
  (:`Pressed`
    (bind _ashsw_game_state_auditorium (cast `HSW_GameState_Auditorium` (`GameplayStatics.GetGameState`))
      (:`then`
        (`HSW_GameState_Auditorium.ServerRPC_SetInterviewee` _ashsw_game_state_auditorium))
      (:`CastFailed`
        (`KismetSystemLibrary.PrintString` "Fail!")))))

(event `ServerPlayAnimation`
  (`self.MulticastPlayAniation`))

(event `Key|R`
  (params (Key :type "Key Structure"))
  ;[1 1 1] Keyboard Binding : R 리셋
  (:`Pressed`
    (bind _ashsw_game_state_auditorium (cast `HSW_GameState_Auditorium` (`GameplayStatics.GetGameState`)))
    (bind _ashsw_bp_audience (cast `/Game/Project/Personal/HSW/Blueprints/HSW_BP_Audience` (`PlayerState.GetPawn` (`|GetArrayItem` (`GameStateBase.PlayerArray` _ashsw_game_state_auditorium) 1))))
    (`HSW_ThirdPersonCharacter.ServerFeverReset` _ashsw_bp_audience)))

(event `Key|One`
  (params (Key :type "Key Structure"))
  ;[1 1 1] 이펙트 생성
  (:`Pressed`
    (`|SpawnActorFromClass` "/Game/Project/Personal/JSW/04_NS_JSW/FeverVFX/BP_VFX-Fever-A_JSW.BP_VFX-Fever-A_JSW_C" (`self.Transform`) "Undefined" "MultiplyWithRoot" null null)))

(event `Key|Q`
  (params (Key :type "Key Structure"))
  (bind _dummies (`self.Dummies`))
  (:`Pressed`
    (`/Engine/EditorBlueprintResources/StandardMacros.FlipFlop`
      (:`A`
        (for _array_element _dummies
          (set `Dummy_KMK.bCanThrow` true _array_element)))
      (:`B`
        (for _array_element_2 _dummies
          (set `Dummy_KMK.bCanThrow` false _array_element_2))))))

(fn `UserConstructionScript`
  (`parent.UserConstructionScript`))
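; Audience character Blueprint that supplies cosmetic reactions and triggers for a sound and cutscenes.
; BeginPlay gives the locally controlled host the "Virtual" capsule collision profile and everyone else "Player"; Tick spins a visible VIP object at a frame-rate-dependent speed.
; Events restart a mesh-rolling ShakeBody timeline, play the YouAndI sound, or start one of three level sequences.
; Throw, ball-spawn and emoji-fade logic is unwired or empty.
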(event `self.ReceiveBeginPlay`
  (if (and (`self.HasAuthority`) (`self.IsLocallyControlled`))
    (`PrimitiveComponent.SetCollisionProfileName` (`self.CapsuleComponent`) "Virtual" true)
    (else
      (`PrimitiveComponent.SetCollisionProfileName` (`self.CapsuleComponent`) "Player" true))))

(event `FadeInImogiBlueprint_1`)

(event `self.ReceiveTick`
  (params (DeltaSeconds :type "Float (single-precision)"))
  (if (`SceneComponent.IsVisible` (`self.VIPObject`))
    (`SceneComponent.K2_AddRelativeRotation` (`self.VIPObject`) (`KismetMathLibrary.MakeRotator` 0.0 0.0 (+ DeltaSeconds 10.0)) false false)))

(event `Key|G`
  (params (Key :type "Key Structure")))

(event `PlayWav`
  (`GameplayStatics.PlaySound2D` "/Game/Project/CommonFile/SFX/YouAndI.YouAndI" 1.0 1.0 0.0 null null))

(event `ShakeBodyBlueprint_1`)

(event `ShakeBodyBlueprint_2`
  (bind (_direction _newtrack_3 _newtrack_0) (`Timeline|ShakeBody` :!via `PlayFromStart` :!label _label)
    (:`Update`
      (`SceneComponent.K2_SetRelativeRotation` (`self.Mesh`) (`KismetMathLibrary.MakeRotator` (`KismetMathLibrary.Lerp` -20.0 50.0 _newtrack_3) 0.0 -90.0) false false))
    (:`Finished`
      (`SceneComponent.K2_SetRelativeRotation` (`self.Mesh`) (`KismetMathLibrary.MakeRotator` 0.0 0.0 -90.0) false false))))

(event `self.ShakeBodyBlueprint`
  (goto _label :!via `PlayFromStart`))

(event `PlaySeqeunce`
  (bind _outactor (`LevelSequencePlayer.CreateLevelSequencePlayer` "/Game/Project/Personal/HSW/LS_BetaStart01.LS_BetaStart01"))
  (`MovieSceneSequencePlayer.Play` (`LevelSequenceActor.SequencePlayer` _outactor)))

(event `PlaySeqeunce2`
  (bind _outactor (`LevelSequencePlayer.CreateLevelSequencePlayer` "/Game/Project/Personal/HSW/TimeGoesOn.TimeGoesOn"))
  (`MovieSceneSequencePlayer.Play` (`LevelSequenceActor.SequencePlayer` _outactor)))

(event `PlaySequence3`
  (bind _outactor (`LevelSequencePlayer.CreateLevelSequencePlayer` "/Game/Project/Personal/HSW/Landing.Landing"))
  (`MovieSceneSequencePlayer.Play` (`LevelSequenceActor.SequencePlayer` _outactor)))

(fn `UserConstructionScript`)
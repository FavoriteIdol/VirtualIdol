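; Test character Blueprint for proximity-style voice chat, with F as a push-to-talk key that toggles speaking through console commands.
; BeginPlay picks a capsule collision profile by authority and local control, then adds a VOIP talker, retrying until PlayerState is valid.
; It registers the talker, attaches its settings to the capsule, sets the mic threshold and enables local loopback.
; A timeline event shakes the mesh's roll; other event stubs and throwing logic are inactive.
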(event `self.ReceiveBeginPlay`
  (`|ExecutionSequence`
    (:`then_0`
      (if (and (`self.HasAuthority`) (`self.IsLocallyControlled`))
        (`PrimitiveComponent.SetCollisionProfileName` (`self.CapsuleComponent`) "Virtual" true)
        (else
          (`PrimitiveComponent.SetCollisionProfileName` (`self.CapsuleComponent`) "Player" true))))
    (:`then_1`
      (bind _returnvalue (`AddComponent|NODE_AddVOIPTalker-0`))
      (bind _output_get (set `self.VOIP REF` _returnvalue))
      (`/Engine/EditorBlueprintResources/StandardMacros.IsValid` (`self.PlayerState`) :!label _label
        (:`Is Valid`
          (`VOIPTalker.RegisterWithPlayerState` _output_get (`self.PlayerState`))
          (`VOIPStatics.SetMicThreshold` -20.0)
          (set `VOIPTalker.Settings` (make `VoiceSettings` (`self.CapsuleComponent`)) (`self.VOIP REF`))
          (if (`self.IsLocallyControlled`)
            (`KismetSystemLibrary.ExecuteConsoleCommand` "OSS.VoiceLoopback 1" null)
            (`KismetSystemLibrary.PrintString` "Hello")))
        (:`Is Not Valid`
          (`KismetSystemLibrary.Delay` 0.2)
          (goto _label))))))

(event `FadeInImogiBlueprint_1`)

(event `Key|G`
  (params (Key :type "Key Structure")))

(event `ShakeBodyBlueprint_1`)

(event `ShakeBodyBlueprint_2`
  (bind (_direction _newtrack_3 _newtrack_0) (`Timeline|ShakeBody` :!via `PlayFromStart`)
    (:`Update`
      (`SceneComponent.K2_SetRelativeRotation` (`self.Mesh`) (`KismetMathLibrary.MakeRotator` (`KismetMathLibrary.Lerp` -20.0 50.0 _newtrack_3) 0.0 -90.0) false false))
    (:`Finished`
      (`SceneComponent.K2_SetRelativeRotation` (`self.Mesh`) (`KismetMathLibrary.MakeRotator` 0.0 0.0 -90.0) false false))))

(event `self.MICSettingBlueprint`)

(event `self.MICOnBlueprint`)

(event `self.MICOffBlueprint`)

(event `Key|F`
  (params (Key :type "Key Structure"))
  (:`Pressed`
    (`KismetSystemLibrary.PrintString` "On")
    (`KismetSystemLibrary.ExecuteConsoleCommand` "ToggleSpeaking 1" null))
  (:`Released`
    (`KismetSystemLibrary.PrintString` "Off")
    (`KismetSystemLibrary.ExecuteConsoleCommand` "ToggleSpeaking 0" null)))

(fn `UserConstructionScript`)
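; Character Blueprint for an alpha test, handling collision setup, a body-shake animation and a landing cinematic.
; BeginPlay gives the capsule the "Virtual" profile when authoritative and locally controlled, otherwise "Player".
; Shake events play a timeline that rolls the mesh and resets it when finished, while PlaySeqeunce plays the Landing level sequence.
; Throwing, ball-spawn and emoji fade-in logic remains only as empty events or disconnected nodes.
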(event `PlaySeqeunce`
  (`KismetSystemLibrary.PrintString` "Hello")
  (bind _outactor (`LevelSequencePlayer.CreateLevelSequencePlayer` "/Game/Project/Personal/JJH/Landing.Landing"))
  (`MovieSceneSequencePlayer.Play` (`LevelSequenceActor.SequencePlayer` _outactor)))

(event `FadeInImogiBlueprint_1`
  ;[0.04688 0.04211 0.004427] 쓰레기통
)

(event `self.ReceiveBeginPlay`
  ;[1 1 1] 이름 띄우기
  (if (and (`self.HasAuthority`) (`self.IsLocallyControlled`))
    (`PrimitiveComponent.SetCollisionProfileName` (`self.CapsuleComponent`) "Virtual" true)
    (else
      (`PrimitiveComponent.SetCollisionProfileName` (`self.CapsuleComponent`) "Player" true))))

(event `Key|G`
  (params (Key :type "Key Structure"))
  ;[0.04688 0.04211 0.004427] 쓰레기통
)

(event `ShakeBodyBlueprint_1`
  ;[1 1 1] 몸 흔들기
)

(event `ShakeBodyBlueprint_2`
  ;[1 1 1] 몸 흔들기
  (bind (_direction _newtrack_3 _newtrack_0) (`Timeline|ShakeBody` :!via `PlayFromStart` :!label _label)
    (:`Update`
      (`SceneComponent.K2_SetRelativeRotation` (`self.Mesh`) (`KismetMathLibrary.MakeRotator` (`KismetMathLibrary.Lerp` -20.0 50.0 _newtrack_3) 0.0 -90.0) false false))
    (:`Finished`
      (`SceneComponent.K2_SetRelativeRotation` (`self.Mesh`) (`KismetMathLibrary.MakeRotator` 0.0 0.0 -90.0) false false))))

(event `self.ShakeBodyBlueprint`
  ;[1 1 1] 몸 흔들기
  (goto _label :!via `PlayFromStart`))

(event `Key|One`
  (params (Key :type "Key Structure")))

(fn `UserConstructionScript`)
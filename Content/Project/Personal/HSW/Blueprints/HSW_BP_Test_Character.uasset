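; Test character Blueprint whose only working behavior is a body-shake animation.
; ShakeBodyBlueprint plays a timeline that rocks the mesh's roll, then restores its upright rotation when finished.
; FadeInImogiBlueprint_1 is an empty event, and the construction script does nothing.
; Leftover unconnected nodes cover object throwing, ball spawning, movement disabling, an emoji fade-in, a concert cheat and debug prints, none of which run.
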(event `FadeInImogiBlueprint_1`)

(event `Key|G`
  (params (Key :type "Key Structure")))

(event `self.ShakeBodyBlueprint`
  (bind (_direction _newtrack_3 _newtrack_0) (`Timeline|ShakeBody` :!via `PlayFromStart`)
    (:`Update`
      (`SceneComponent.K2_SetRelativeRotation` (`self.Mesh`) (`KismetMathLibrary.MakeRotator` (`KismetMathLibrary.Lerp` -20.0 50.0 _newtrack_3) 0.0 -90.0) false false))
    (:`Finished`
      (`SceneComponent.K2_SetRelativeRotation` (`self.Mesh`) (`KismetMathLibrary.MakeRotator` 0.0 0.0 -90.0) false false))))

(event `Key|C`
  (params (Key :type "Key Structure")))

(fn `UserConstructionScript`)
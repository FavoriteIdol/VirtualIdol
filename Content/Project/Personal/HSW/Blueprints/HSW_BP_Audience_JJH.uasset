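; Audience character for a concert that drives its skeletal mesh from received motion data through a Control Rig.
; The rig takes initial bone transforms from the mesh; on a locally controlled authority, received control transforms are applied in world space, offset by the mesh's starting location, with debug prints.
; A timeline rocks the mesh for a body shake, and C triggers a cheat concert start.
; Throwing and emoji fade logic is left disconnected.
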(event `FadeInImogiBlueprint_1`)

(event `Key|G`
  (params (Key :type "Key Structure")))

(event `Key|C`
  (params (Key :type "Key Structure"))
  (:`Pressed`
    (if (and (`self.HasAuthority`) (`self.IsLocallyControlled`))
      (`AudienceServerComponent_KMK.CheatStartConcert` (`self.AudienceServerComponent_KMK`)))))

(event `self.ShakeBodyBlueprint`
  (bind (_direction _newtrack_3 _newtrack_0) (`Timeline|ShakeBody` :!via `PlayFromStart`)
    (:`Update`
      (`SceneComponent.K2_SetRelativeRotation` (`self.Mesh`) (`KismetMathLibrary.MakeRotator` (`KismetMathLibrary.Lerp` -20.0 50.0 _newtrack_3) 0.0 -90.0) false false))
    (:`Finished`
      (`SceneComponent.K2_SetRelativeRotation` (`self.Mesh`) (`KismetMathLibrary.MakeRotator` 0.0 0.0 -90.0) false false))))

(event `self.ControlRig.OnPreConstructionDelegate`
  (params (Component :type "ControlRigComponent Object Reference"))
  (bind _skeletalmesh (`self.SkeletalMesh`))
  (for _array_element (`SceneComponent.GetAllSocketNames` _skeletalmesh)
    (if (`SceneComponent.DoesSocketExist` _skeletalmesh _array_element)
      (`ControlRigComponent.SetInitialBoneTransform` (`self.ControlRig`) _array_element (`SceneComponent.GetSocketTransform` _skeletalmesh _array_element "RTS_Component") "ComponentSpace" true))))

(event `self.ControlRig.OnPostInitializeDelegate`
  (params (Component :type "ControlRigComponent Object Reference"))
  (`ControlRigComponent.AddMappedCompleteSkeletalMesh` (`self.ControlRig`) (`self.SkeletalMesh`) "Output"))

(event `self.ReceiveBeginPlay`
  (bind _bp_motionreceivercomponent (`self.BP_MotionReceiverComponent`))
  (set `self.MeshInitialLocation` (`SceneComponent.K2_GetComponentLocation` (`self.SkeletalMesh`)))
  (add `/ReMoCapp/Components/BP_MotionReceiverComponent.OnControlTransformReceived` _bp_motionreceivercomponent (delegate `ControlTransformReceived`))
  (add `/ReMoCapp/Components/BP_MotionReceiverComponent.OnRetrievingControlsDataFinished` _bp_motionreceivercomponent (delegate `RetrievingControlsDataFinished`)))

(event `RetrievingControlsDataFinished`
  (`ControlRigComponent.Update` (`self.ControlRig`) 0.0))

(event `ControlTransformReceived`
  (params (ControlIndex :type Integer) (ControlTransform :type "Transform Structure"))
  (if (and (`self.HasAuthority`) (`self.IsLocallyControlled`))
    (`self.1231234` ControlIndex ControlTransform)))

(event `1231234`
  (params (NewParam :type Integer) (NewParam2 :type "Transform Structure"))
  (bind _controlrig (`self.ControlRig`))
  (bind _returnvalue (`KismetMathLibrary.MakeTransform` (+ (.location NewParam2) (`self.MeshInitialLocation`)) (.rotation NewParam2) (.scale NewParam2)))
  (`/Engine/EditorBlueprintResources/StandardMacros.IsValid` _controlrig
    (:`Is Valid`
      (`ControlRigComponent.SetControlTransform` _controlrig (`|GetArrayItem` (`self.Rig Control Names`) NewParam) _returnvalue "WorldSpace")
      (`KismetSystemLibrary.PrintString` (`KismetSystemLibrary.GetDisplayName` _controlrig) true true (struct :`R` 1.0 :`B` 0.223804 :`A` 1.0))
      (`KismetSystemLibrary.PrintString` (`KismetStringLibrary.Conv_TransformToString` _returnvalue) true true (struct :`R` 1.0 :`B` 0.223804 :`A` 1.0)))))

(fn `UserConstructionScript`)
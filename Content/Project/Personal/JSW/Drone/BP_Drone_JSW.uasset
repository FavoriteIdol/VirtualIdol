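; BP_Drone_JSW is an ambient drone that wanders within a fixed area while bobbing, spinning its propellers and aiming a light beam.
; BeginPlay picks a random XY target, and Tick picks a new one whenever a ten-second timer elapses.
; Each Tick interpolates toward that target with a time-based sine offset on current height, rotates four propeller origins and turns the beam toward Point.
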(event `self.ReceiveBeginPlay`
  (set `self.targetPos` (`KismetMathLibrary.MakeVector` (`KismetMathLibrary.RandomFloatInRange` -340.0 -1220.0) (`KismetMathLibrary.RandomFloatInRange` -1000.0 1000.0))))

(event `self.ReceiveTick`
  (params (DeltaSeconds :type "Float (single-precision)"))
  (bind (_returnvalue_x _returnvalue_y _returnvalue_z) (`KismetMathLibrary.BreakVector` (`self.K2_GetActorLocation`)))
  (bind (_targetpos_x _targetpos_y) (`KismetMathLibrary.BreakVector` (`self.targetPos`)))
  (bind _s_ev_simplelightbeam_03 (`self.S_EV_SimpleLightBeam_03`))
  (`SceneComponent.K2_AddLocalRotation` (`self.SM_Propeller-Origin2`) (`KismetMathLibrary.MakeRotator` 0.0 0.0 (* DeltaSeconds (`self.proSpeed`))) false false)
  (`SceneComponent.K2_AddLocalRotation` (`self.SM_Propeller-Origin1`) (`KismetMathLibrary.MakeRotator` 0.0 0.0 (* DeltaSeconds (`self.proSpeed`))) false false)
  (`SceneComponent.K2_AddLocalRotation` (`self.SM_Propeller-Origin3`) (`KismetMathLibrary.MakeRotator` 0.0 0.0 (* DeltaSeconds (`self.proSpeed`))) false false)
  (`SceneComponent.K2_AddLocalRotation` (`self.SM_Propeller-Origin`) (`KismetMathLibrary.MakeRotator` 0.0 0.0 (* DeltaSeconds (`self.proSpeed`))) false false)
  (`SceneComponent.K2_SetRelativeRotation` _s_ev_simplelightbeam_03 (`KismetMathLibrary.FindLookAtRotation` (`SceneComponent.K2_GetComponentLocation` _s_ev_simplelightbeam_03) (`self.point`)) false false)
  (`self.K2_SetActorLocation` (`KismetMathLibrary.VInterpTo` (`self.K2_GetActorLocation`) (`KismetMathLibrary.MakeVector` _targetpos_x _targetpos_y (+ _returnvalue_z (* (`KismetMathLibrary.DegSin` (* (`self.freq`) (`KismetSystemLibrary.GetGameTimeInSeconds`))) (`self.amp`)))) (`GameplayStatics.GetWorldDeltaSeconds`) 2.0))
  (set `self.timer` (+ DeltaSeconds (`self.timer`)))
  (if (> (`self.timer`) 10.0)
    (set `self.targetPos` (`KismetMathLibrary.MakeVector` (`KismetMathLibrary.RandomFloatInRange` -340.0 -1220.0) (`KismetMathLibrary.RandomFloatInRange` -1000.0 1000.0)))
    (set `self.timer` 0.0)))

(fn `UserConstructionScript`)
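; Moving-head spotlight actor that continuously turns toward the first actor tagged "Virtual", found at BeginPlay.
; The construction script applies the configured light intensity and the starting yoke and head rotations.
; On Tick, MoveLight lerps both meshes' relative rotations toward a world-space look-at rotation, using DeltaSeconds as alpha.
; A five-second timer only skips one update when it resets, and the cached roll and yaw go unused.
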(event `self.ReceiveBeginPlay`
  (bind (_returnvalue_roll _returnvalue_pitch _returnvalue_yaw) (`KismetMathLibrary.BreakRotator` (`self.K2_GetActorRotation`)))
  (set `self.x` _returnvalue_roll)
  (set `self.z` _returnvalue_yaw)
  (bind _outactors (`GameplayStatics.GetAllActorsOfClassWithTag` "/Script/Engine.Actor" "Virtual"))
  (set `self.virtual` (`|GetArrayItem` _outactors)))

(event `self.ReceiveTick`
  (params (DeltaSeconds :type "Float (single-precision)"))
  (`self.MoveLight` DeltaSeconds))

(fn `MoveLight`
  (params (alpha :type "Float (double-precision)"))
  (bind _sm_movinghead_head (`self.SM_MovingHead_Head`))
  (bind _returnvalue (`KismetMathLibrary.FindLookAtRotation` (`self.K2_GetActorLocation`) (`self.K2_GetActorLocation` (`self.virtual`))))
  (bind _output_get (set `self.AlphaTime` (+ alpha (`self.AlphaTime`))))
  (if (< _output_get 5.0)
    (`SceneComponent.K2_SetRelativeRotation` (`self.SM_MovingHead_Yoke`) (`KismetMathLibrary.RLerp` (`SceneComponent.RelativeRotation` (`self.SM_MovingHead_Yoke`)) _returnvalue alpha) false false)
    (`SceneComponent.K2_SetRelativeRotation` _sm_movinghead_head (`KismetMathLibrary.RLerp` (`SceneComponent.RelativeRotation` _sm_movinghead_head) _returnvalue alpha) false false)
    (else
      (set `self.AlphaTime` 0.0))))

(fn `UserConstructionScript`
  (`LightComponent.SetIntensity` (`self.SpotLight`) (`self.lightIntensity`))
  (`SceneComponent.K2_SetRelativeRotation` (`self.SM_MovingHead_Yoke`) (`self.ratationYoke`) false false)
  (`SceneComponent.K2_SetRelativeRotation` (`self.SM_MovingHead_Head`) (`self.rotationHead`) false false))
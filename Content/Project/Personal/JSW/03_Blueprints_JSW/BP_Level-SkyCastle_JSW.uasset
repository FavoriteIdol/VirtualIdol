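; BP_Level-SkyCastle_JSW is a Sky Castle level Blueprint that animates rotating scenery components.
; Every Tick rotates five GoseguLevel components around their local pitch axis, each with its own speed variable.
; The moon component turns in yaw through a relative rotation at its own speed.
; All rotation is scaled by DeltaSeconds for frame-rate independence, and BeginPlay and the construction script do nothing.
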(event `self.ReceiveTick`
  (params (DeltaSeconds :type "Float (single-precision)"))
  (`SceneComponent.K2_AddLocalRotation` (`self.GoseguLevel_B_GoseguLevel-0`) (`KismetMathLibrary.MakeRotator` 0.0 (* DeltaSeconds (`self.jswRotationSpeed-0`))) false false)
  (`SceneComponent.K2_AddLocalRotation` (`self.GoseguLevel_B_GoseguLevel-1`) (`KismetMathLibrary.MakeRotator` 0.0 (* DeltaSeconds (`self.jswRotationSpeed-1`))) false false)
  (`SceneComponent.K2_AddLocalRotation` (`self.GoseguLevel_B_GoseguLevel-2`) (`KismetMathLibrary.MakeRotator` 0.0 (* DeltaSeconds (`self.jswRotationSpeed-2`))) false false)
  (`SceneComponent.K2_AddLocalRotation` (`self.GoseguLevel_B_GoseguLevel-3`) (`KismetMathLibrary.MakeRotator` 0.0 (* DeltaSeconds (`self.jswRotationSpeed-3`))) false false)
  (`SceneComponent.K2_AddLocalRotation` (`self.GoseguLevel_B_GoseguLevel-4`) (`KismetMathLibrary.MakeRotator` 0.0 (* DeltaSeconds (`self.jswRotationSpeed-4`))) false false)
  (`SceneComponent.K2_AddRelativeRotation` (`self.jswMoon`) (`KismetMathLibrary.MakeRotator` 0.0 0.0 (* DeltaSeconds (`self.jswMoonSpeed`))) false false))

(fn `UserConstructionScript`)